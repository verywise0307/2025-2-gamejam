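; BP_Seashell2 is a seashell Blueprint that tracks a directional sliding state driven by up, down, left and right input.
; Each press sets the direction and starts sliding, unless it repeats the last accepted direction.
; Two box components end sliding on overlap, one for vertical directions and one for horizontal.
; The graph only sets state variables, with no movement logic and an empty Tick.
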(event OnComponentBeginOverlap(updownBox)
  (params (OverlappedComponent :type Primitive%20Component%20Object%20Reference) (OtherActor :type Actor%20Object%20Reference) (OtherComp :type Primitive%20Component%20Object%20Reference) (OtherBodyIndex :type Integer) (bFromSweep :type Boolean) (SweepResult :type Hit%20Result%20Structure%20%28by%20ref%29))
  (bind _direction (Variables|Default|Getdirection))
  (if (or (== _direction 0) (== _direction 1))
    (Variables|Default|Setissliding false)))

(event OnComponentBeginOverlap(leftrightBox)
  (params (OverlappedComponent :type Primitive%20Component%20Object%20Reference) (OtherActor :type Actor%20Object%20Reference) (OtherComp :type Primitive%20Component%20Object%20Reference) (OtherBodyIndex :type Integer) (bFromSweep :type Boolean) (SweepResult :type Hit%20Result%20Structure%20%28by%20ref%29))
  (bind _direction (Variables|Default|Getdirection))
  (if (or (== _direction 2) (== _direction 3))
    (Variables|Default|Setissliding false)))

(event EventBeginPlay)

(event Collision|EventActorBeginOverlap
  (params (OtherActor :type Actor%20Object%20Reference)))

(event EventTick
  (params (DeltaSeconds :type Float%20%28single-precision%29)))

(event Input|ActionEvents|InputActionup
  (params (Key :type Key%20Structure :default "None"))
  ;[1 1 1] WASD
  (:Pressed
    (if (!= (Variables|Default|Getpredirection) 0)
      (Variables|Default|Setissliding true)
      (Variables|Default|Setdirection 0)
      (Variables|Default|Setpredirection 0))))

(event Input|ActionEvents|InputActiondown
  (params (Key :type Key%20Structure :default "None"))
  ;[1 1 1] WASD
  (:Pressed
    (if (!= (Variables|Default|Getpredirection) 1)
      (Variables|Default|Setissliding true)
      (Variables|Default|Setdirection 1)
      (Variables|Default|Setpredirection 1))))

(event Input|ActionEvents|InputActionleft
  (params (Key :type Key%20Structure :default "None"))
  ;[1 1 1] WASD
  (:Pressed
    (if (!= (Variables|Default|Getpredirection) 2)
      (Variables|Default|Setissliding true)
      (Variables|Default|Setdirection 2)
      (Variables|Default|Setpredirection 2))))

(event Input|ActionEvents|InputActionright
  (params (Key :type Key%20Structure :default "None"))
  ;[1 1 1] WASD
  (:Pressed
    (if (!= (Variables|Default|Getpredirection) 3)
      (Variables|Default|Setissliding true)
      (Variables|Default|Setdirection 3)
      (Variables|Default|Setpredirection 3))))

(fn ConstructionScript)