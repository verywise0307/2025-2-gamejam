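; BP_breakableWall is a wall that the seashell player actor (BP_Seashell3) smashes by hitting it with its mesh.
; A Sphere overlap decrements the seashell's bubble count, syncs it to the game instance and calls BreakAndContinue.
; It then destroys every wall sharing its Code, with a crash sound, so segments break as a group.
; The initbreaking event makes mesh and sphere ignore GameTraceChannel1 when Topview and Canbreak hold, otherwise block it.
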(event OnComponentBeginOverlap(Sphere)
  (params (OverlappedComponent :type Primitive%20Component%20Object%20Reference) (OtherActor :type Actor%20Object%20Reference) (OtherComp :type Primitive%20Component%20Object%20Reference) (OtherBodyIndex :type Integer) (bFromSweep :type Boolean) (SweepResult :type Hit%20Result%20Structure%20%28by%20ref%29))
  (bind _asbp_seashell_3 (Utilities|Casting|CastToBP_Seashell3 OtherActor))
  (if (== OtherComp (Variables|/Game/Spiral_Seashell/BP_Seashell3.BP_Seashell3_C|GetSeashellMesh _asbp_seashell_3))
    (bind _result (Math|Integer|DecrementInt (Variables|/Game/Spiral_Seashell/BP_Seashell3.BP_Seashell3_C|Getbubblecount _asbp_seashell_3))
      (:%20%20
        (bind _asseashell_gameinstance (Utilities|Casting|CastToSeashell_gameinstance (Game|GetGameInstance)))
        (Variables|/Game/Spiral_Seashell/Seashell_gameinstance.Seashell_gameinstance_C|Setbubblecount _asseashell_gameinstance _result)
        (Default|InitBubble _asseashell_gameinstance)
        (Default|BreakandContinue _asbp_seashell_3)
        (bind _outactors (Actor|GetAllActorsOfClass "BP_breakableWall_C"))
        (for _array_element _outactors
          (if (== (Variables|BP_breakableWall_C|Getcode _array_element) (Variables|Default|Getcode))
            (Audio|PlaySound2D "/Game/assets/새_폴더_(4)/box_crash.box_crash" 1.0 1.0 0.0 0 0)
            (Actor|DestroyActor _array_element)))))))

(event Custom|initbreaking
  (if (and (Variables|Default|Gettopview) (Variables|Default|Getcanbreak))
    (Collision|SetCollisionResponsetoChannel (Variables|Default|GetStaticMesh) "ECC_GameTraceChannel1" "ECR_Ignore")
    (Collision|SetCollisionResponsetoChannel (Variables|Default|GetSphere) "ECC_GameTraceChannel1" "ECR_Ignore")
    (else
      (Collision|SetCollisionResponsetoChannel (Variables|Default|GetStaticMesh) "ECC_GameTraceChannel1" "ECR_Block")
      (Collision|SetCollisionResponsetoChannel (Variables|Default|GetSphere) "ECC_GameTraceChannel1" "ECR_Block"))))

(event EventBeginPlay)

(event Collision|EventActorBeginOverlap
  (params (OtherActor :type Actor%20Object%20Reference)))

(event EventTick
  (params (DeltaSeconds :type Float%20%28single-precision%29)))

(fn ConstructionScript)