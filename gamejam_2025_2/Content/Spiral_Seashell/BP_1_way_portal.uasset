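; BP_1_way_portal is a one-way teleport portal for the BP_Seashell3 player pawn in the Spiral Seashell game.
; When the player overlaps its mesh and the portal is marked Start, it searches all portals for one with the same Code and an opposite ToThirdview flag.
; It sets that portal's location as the seashell's TPpoint and calls the pawn's TP, unless a teleport is already in progress.
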(event OnComponentBeginOverlap(StaticMesh)
  (params (OverlappedComponent :type Primitive%20Component%20Object%20Reference) (OtherActor :type Actor%20Object%20Reference) (OtherComp :type Primitive%20Component%20Object%20Reference) (OtherBodyIndex :type Integer) (bFromSweep :type Boolean) (SweepResult :type Hit%20Result%20Structure%20%28by%20ref%29))
  (bind _asbp_seashell_3 (Utilities|Casting|CastToBP_Seashell3 (Game|Player|GetPlayerPawn 0)))
  (if (== _asbp_seashell_3 OtherActor)
    (bind _outactors (Actor|GetAllActorsOfClass "BP_1_way_portal_C"))
    (for _array_element _outactors
      (if (Math|Boolean|ANDBoolean (== (Variables|BP_1_way_portal_C|Getcode _array_element) (Variables|Default|Getcode)) (!= (Variables|BP_1_way_portal_C|GettoThirdview _array_element) (Variables|Default|GettoThirdview)) (Variables|Default|Getstart))
        (Variables|/Game/Spiral_Seashell/BP_Seashell3.BP_Seashell3_C|SetTPpoint _asbp_seashell_3 (Transformation|GetActorLocation _array_element))
        (if (not (Variables|/Game/Spiral_Seashell/BP_Seashell3.BP_Seashell3_C|Getisteleporting _asbp_seashell_3))
          (Default|TP _asbp_seashell_3))))))

(event EventBeginPlay)

(event Collision|EventActorBeginOverlap
  (params (OtherActor :type Actor%20Object%20Reference)))

(event EventTick
  (params (DeltaSeconds :type Float%20%28single-precision%29)))

(fn ConstructionScript)