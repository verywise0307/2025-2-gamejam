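; BP_airbubble is a collectible air bubble actor that the BP_Seashell3 actor picks up on contact.
; When its StaticMesh begins overlapping that seashell's SeashellMesh component specifically, it increments the seashell's Bubblecount.
; It then copies the count to Seashell_gameinstance, calls InitBubble there and destroys itself.
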(event OnComponentBeginOverlap(StaticMesh)
  (params (OverlappedComponent :type Primitive%20Component%20Object%20Reference) (OtherActor :type Actor%20Object%20Reference) (OtherComp :type Primitive%20Component%20Object%20Reference) (OtherBodyIndex :type Integer) (bFromSweep :type Boolean) (SweepResult :type Hit%20Result%20Structure%20%28by%20ref%29))
  (bind _asbp_seashell_3 (Utilities|Casting|CastToBP_Seashell3 OtherActor))
  (if (== OtherComp (Variables|/Game/Spiral_Seashell/BP_Seashell3.BP_Seashell3_C|GetSeashellMesh _asbp_seashell_3))
    (bind _result (Math|Integer|IncrementInt (Variables|/Game/Spiral_Seashell/BP_Seashell3.BP_Seashell3_C|Getbubblecount _asbp_seashell_3))
      (:%20%20
        (bind _asseashell_gameinstance (Utilities|Casting|CastToSeashell_gameinstance (Game|GetGameInstance)))
        (Variables|/Game/Spiral_Seashell/Seashell_gameinstance.Seashell_gameinstance_C|Setbubblecount _asseashell_gameinstance _result)
        (Default|InitBubble _asseashell_gameinstance)
        (Actor|DestroyActor)))))

(event EventBeginPlay)

(event Collision|EventActorBeginOverlap
  (params (OtherActor :type Actor%20Object%20Reference)))

(event EventTick
  (params (DeltaSeconds :type Float%20%28single-precision%29)))

(fn ConstructionScript)